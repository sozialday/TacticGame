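; Player cursor actor that carries a separate CursorPointer visual, spawned on BeginPlay and attached above it.
; Events forward height changes and resets to the pointer, which handles its own Z movement.
; Test keys box-trace for pawns at the cursor: V grants a large XP amount to the UnitCharacterBase hit, and Ctrl+V damages it.
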(event EventBeginPlay
  ;[1 0.7972 0.271 0.5 30] Cursor Actor [Visualiser]
  ;;[0.06771 0.06771 0.06771] Spawns and attaches the Cursor VISUAL to the actual Cursor
  (bind _returnvalue (Game|SpawnActorfromClass "/Script/TacticGame.CursorPointer" (Math|Transform|MakeTransform "0, 0, 0" "0, 0, 0" "1.000000,1.000000,1.000000") "AlwaysSpawn" "MultiplyWithRoot" 0 0))
  (bind _output_get (Variables|Default|SetPointer _returnvalue))
  (Transformation|AttachActorToActor _output_get self "None" "SnapToTarget" "SnapToTarget" "SnapToTarget" true)
  (Transformation|SetActorRelativeLocation _output_get "0.000000,0.000000,375.000000"))

(event EventSetCursorArrowDistanceSpeed
  (params (NewZTarget :type Float%20%28single-precision%29))
  ;[1 0.7972 0.271 0.5 30] Cursor Actor [Visualiser]
  ;;[0.15 0.15 0.15 0.5] Cursor Z Offset Adjustment
  (Class|CursorPointer|ChangeZTranslations (Variables|Default|GetPointer) 0.0 NewZTarget true true))

(event EventResetCursorArrowDistance
  ;[1 0.7972 0.271 0.5 30] Cursor Actor [Visualiser]
  ;;[0.15 0.15 0.15 0.5] Cursor Z Offset Adjustment
  (Class|CursorPointer|ResettoBasic (Variables|Default|GetPointer)))

(event Input|KeyboardEvents|CtrlV
  (params (Key :type Key%20Structure :default "None"))
  (bind _returnvalue (Transformation|GetActorLocation))
  ;[0.15 0.15 0.15 0.5] Test Damage Application
  (:Pressed
    (bind (_outhit _returnvalue_2) (Class|KismetSystemLibrary|BoxTraceSingleforObjects _returnvalue _returnvalue "90.000000,90.000000,350.000000" "0, 0, 0" (Utilities|Array|MakeArray "ObjectTypeQuery3") false 0 "ForDuration" true))
    (if _returnvalue_2
      (Utilities|IsValid (.HitActor (Collision|BreakHitResult _outhit))
        (:Is%20Valid
          (bind _asunit_character_base (Utilities|Casting|CastToUnitCharacterBase (.HitActor (Collision|BreakHitResult _outhit))))
          (Game|Damage|ApplyDamage _asunit_character_base 1e+01 0 0))))))

(event Input|KeyboardEvents|V
  (params (Key :type Key%20Structure :default "None"))
  (bind _returnvalue (Transformation|GetActorLocation))
  ;[0.15 0.15 0.15 0.5] Test Damage Application
  (:Pressed
    (bind (_outhit _returnvalue_2) (Class|KismetSystemLibrary|BoxTraceSingleforObjects _returnvalue _returnvalue "90.000000,90.000000,350.000000" "0, 0, 0" (Utilities|Array|MakeArray "ObjectTypeQuery3") false 0 "ForDuration" true))
    (if _returnvalue_2
      (Utilities|IsValid (.HitActor (Collision|BreakHitResult _outhit))
        (:Is%20Valid
          (bind _asunit_character_base (Utilities|Casting|CastToUnitCharacterBase (.HitActor (Collision|BreakHitResult _outhit))))
          (Class|UnitStatsComponent|AddXP (Variables|/Script/TacticGame.UnitCharacterBase|GetUnitStats _asunit_character_base) 5e+05))))))

(fn ConstructionScript)